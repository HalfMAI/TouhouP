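; BP_ActionManager is an actor that spawns and keeps track of a controlled action point.
; On BeginPlay it spawns an ActionPointClass actor at InitControllPoint and stores it as CurControlledPoint.
; MoveFoward teleports that point along its local axes by FowardDir times MoveDistance, without sweeping.
; The delayed MoveFoward call in the event graph is disconnected, so nothing in this Blueprint moves the point at runtime.
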(event `self.ReceiveBeginPlay`
  (`self.SpawnActionPoint` (`KismetMathLibrary.MakeTransform` (`self.InitControllPoint`))))

(event `self.ReceiveTick`
  (params (DeltaSeconds :type "Float (single-precision)")))

(fn `MoveFoward`
  (`self.K2_AddActorLocalOffset` (`self.CurControlledPoint`) (* (`self.FowardDir`) (`self.MoveDistance`)) false true))

(fn `SpawnActionPoint`
  (params (SpawnTransform :type "Transform Structure (by ref)"))
  (bind _returnvalue (`|SpawnActorFromClass` (`self.ActionPointClass`) SpawnTransform "AdjustIfPossibleButAlwaysSpawn" "OverrideRootScale" null null))
  (set `self.CurControlledPoint` _returnvalue))

(fn `UserConstructionScript`)