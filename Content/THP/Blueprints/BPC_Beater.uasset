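; Rhythm component that runs a looping beat timer at a set BPM and grades the timing of presses against the beat.
; Each tick advances a wrapping beat index and broadcasts an OnBeat event with BPM and half-beat length.
; CheckBeatPressType assigns presses to the current or next beat by timer elapsed time, grading them against windows derived from the half-beat.
; A repeat press on either beat gets the same grade as the outermost window.
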(event `self.ReceiveBeginPlay`
  (`self.Init`)
  (bind _returnvalue (`KismetSystemLibrary.K2_SetTimerDelegate` (delegate `_BeatEvent`) (`self.BeatDeltaTime`) true))
  (set `self.BeatTimmer` _returnvalue))

(event `_BeatEvent`
  (set `self.LastBeatTime` (`GameplayStatics.GetTimeSeconds`))
  (`self.BeatIndexAdd` true)
  (`self.OnBeatEvent` (`self.BPM`) (`self.HalfBeatDeltaTime`)))

(fn `BeatIndexAdd`
  (params (IsAddMemberIndex :type Boolean :default true))
  (returns (BeatIndex :type Integer))
  (bind _returnvalue (mod (+ (`self.CurrentBeatIndex`) 1) (`self.MaxBeatRange`)))
  (if IsAddMemberIndex
    (bind _output_get (set `self.CurrentBeatIndex` _returnvalue))
    (return _output_get)
    (else
      (return _returnvalue))))

(fn `CheckBeatPressType`
  (locals (CurrentElapsedTime :type "Float (double-precision)"))
  (bind _beatindex (`self.BeatIndexAdd` false))
  (if (or (== (`self.PressedBeatIndex`) (`self.CurrentBeatIndex`)) (== (`self.PressedBeatIndex`) _beatindex))
    (set `self.CurrentBeatType` "NewEnumerator3")
    (return)
    (else
      (set `local.CurrentElapsedTime` (`KismetSystemLibrary.K2_GetTimerElapsedTimeHandle` (`self.BeatTimmer`)))
      (if (< (`local.CurrentElapsedTime`) (`self.HalfBeatDeltaTime`))
        ;[1 1 1] Current Beat
        (set `self.PressedBeatIndex` (`self.CurrentBeatIndex`))
        ;[1 1 1] Set the Beat Type
        (if (< (`local.CurrentElapsedTime`) (`self.PerfectTime`))
          (set `self.CurrentBeatType` "NewEnumerator0")
          (elif (< (`local.CurrentElapsedTime`) (`self.GoodTime`))
            (set `self.CurrentBeatType` "NewEnumerator1")
            (elif (< (`local.CurrentElapsedTime`) (`self.BadTime`))
              (set `self.CurrentBeatType` "NewEnumerator2")
              (elif (< (`local.CurrentElapsedTime`) (`self.MissTime`))
                (set `self.CurrentBeatType` "NewEnumerator3")))))
        (else
          ;[1 1 1] Next Beat
          (bind _beatindex_2 (`self.BeatIndexAdd` false))
          (set `self.PressedBeatIndex` _beatindex_2)
          ;[1 1 1] Set the Beat Type
          (if (> (`local.CurrentElapsedTime`) (- (`self.BeatDeltaTime`) (`self.PerfectTime`)))
            (set `self.CurrentBeatType` "NewEnumerator0")
            (elif (> (`local.CurrentElapsedTime`) (- (`self.BeatDeltaTime`) (`self.GoodTime`)))
              (set `self.CurrentBeatType` "NewEnumerator1")
              (elif (> (`local.CurrentElapsedTime`) (- (`self.BeatDeltaTime`) (`self.BadTime`)))
                (set `self.CurrentBeatType` "NewEnumerator2")
                (elif (> (`local.CurrentElapsedTime`) (- (`self.BeatDeltaTime`) (`self.MissTime`)))
                  (set `self.CurrentBeatType` "NewEnumerator3"))))))))))

(fn `Init`
  (bind _output_get (set `self.BeatDeltaTime` (/ 60.0 (`self.BPM`))))
  (bind _output_get_2 (set `self.HalfBeatDeltaTime` (* _output_get 0.5)))
  (`|ExecutionSequence`
    (:`then_0`
      (bind _returnvalue (* _output_get_2 0.2))
      ;[1 1 1] Set Type Define
      (bind _output_get_3 (set `self.PerfectTime` _returnvalue))
      (bind _returnvalue_2 (* _output_get_2 0.3))
      (bind _output_get_4 (set `self.GoodTime` (+ _output_get_3 _returnvalue_2)))
      (bind _output_get_5 (set `self.BadTime` (+ _output_get_4 _returnvalue_2)))
      (set `self.MissTime` (+ _output_get_5 _returnvalue)))))