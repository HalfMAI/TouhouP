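; PC_StagePlayerController is the stage player controller, forwarding player input to a spectator pawn and a beat timing check.
; On BeginPlay it caches the GM_MainStage game mode and the controlled BP_Spectator pawn.
; The MoveRight axis passes straight to the spectator.
; BeatPressed asks the game mode's BPCBeater component to classify the press and only prints the result as a string.
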(event `self.ReceiveBeginPlay`
  (bind _asgm_main_stage (cast `/Game/THP/Blueprints/GM_MainStage` (`GameplayStatics.GetGameMode`)))
  (set `self.GM_MainStage_Ref` _asgm_main_stage)
  (bind _asbp_spectator (cast `/Game/THP/Blueprints/BP_Spectator` (`self.K2_GetPawn`)))
  (set `self.Spectator` _asbp_spectator))

(event `InputAxis|MoveRight`
  (params (AxisValue :type "Float (single-precision)"))
  (`DefaultPawn.MoveRight` (`self.Spectator`) AxisValue))

(event `InputAction|BeatPressed`
  (params (Key :type "Key Structure"))
  (:`Pressed`
    (bind _currentbeattype (`/Game/THP/Blueprints/BPC_Beater.CheckBeatPressType` (`/Game/THP/Blueprints/GM_MainStage.BPC_Beater` (`self.GM_MainStage_Ref`))))
    (`KismetSystemLibrary.PrintString` (`|GetEnumeratorNameAsString` _currentbeattype))))

(fn `UserConstructionScript`)